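; BP_EnemyBullet is an enemy projectile that damages what it hits and destroys itself.
; On BeginPlay, its Sphere ignores every existing BP_Enemy_Human while moving, so it does not collide with those enemies.
; When the Sphere hits an actor other than its owner, it applies Damage credited to the instigator's controller, then spawns smoke and plays an explosion sound before being destroyed.
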(event OnComponentHit(Sphere)
  (params (HitComponent :type Primitive%20Component%20Object%20Reference) (OtherActor :type Actor%20Object%20Reference) (OtherComp :type Primitive%20Component%20Object%20Reference) (NormalImpulse :type Vector :default "0, 0, 0") (Hit :type Hit%20Result%20Structure%20%28by%20ref%29))
  (bind _returnvalue (Transformation|GetActorLocation))
  (if (!= OtherActor (Components|GetOwner))
    (Game|Damage|ApplyDamage OtherActor (Variables|Default|GetDamage) (Game|GetInstigatorController) self)
    (Effects|SpawnEmitteratLocation "/Game/StarterContent/Particles/P_Smoke_Enemy.P_Smoke_Enemy" _returnvalue)
    (Audio|PlaySoundatLocation "/Game/StarterContent/Audio/Explosion02.Explosion02" _returnvalue "0, 0, 0" 1.0 1.0 0.0 0 0 0 0)
    (Actor|DestroyActor)))

(event EventBeginPlay
  (bind _outactors (Actor|GetAllActorsOfClass "/Game/ThirdPerson/Blueprints/BP_Enemy_Human.BP_Enemy_Human_C"))
  (for _array_element _outactors
    (Collision|IgnoreActorwhenMoving (Variables|Default|GetSphere) _array_element true)))

(fn ConstructionScript)