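; BP_Player_Bullet is a bullet actor, named for the player, that deals fixed damage on contact and then destroys itself.
; On BeginPlay, its sphere collision ignores the owner while moving.
; Blocking hits apply damage only to actors other than the owner, while the overlap handler damages any overlapping actor without that check.
; Both paths credit the instigator's controller, with the bullet as damage causer.
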(event OnComponentHit(SphereCollision)
  (params (HitComponent :type Primitive%20Component%20Object%20Reference) (OtherActor :type Actor%20Object%20Reference) (OtherComp :type Primitive%20Component%20Object%20Reference) (NormalImpulse :type Vector :default "0, 0, 0") (Hit :type Hit%20Result%20Structure%20%28by%20ref%29))
  (if (!= OtherActor (Components|GetOwner))
    (Game|Damage|ApplyDamage OtherActor 1e+01 (Game|GetInstigatorController) self)
    (Actor|DestroyActor)))

(event Custom|OnComponentBeginOverlap_Event
  (params (OverlappedComponent :type Primitive%20Component%20Object%20Reference) (OtherActor :type Actor%20Object%20Reference) (OtherComp :type Primitive%20Component%20Object%20Reference) (OtherBodyIndex :type Integer) (bFromSweep :type Boolean) (SweepResult :type Hit%20Result%20Structure%20%28by%20ref%29))
  (Game|Damage|ApplyDamage OtherActor 1e+01 (Game|GetInstigatorController) self)
  (Actor|DestroyActor))

(event EventBeginPlay
  (Collision|IgnoreActorwhenMoving (Variables|Default|GetSphereCollision) (Components|GetOwner) true))

(fn ConstructionScript)